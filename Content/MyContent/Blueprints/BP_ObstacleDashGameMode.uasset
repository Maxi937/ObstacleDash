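; Game mode for an Obstacle Dash game that respawns the player character at the level's Player Start.
; The GameModeInterface function gets the location of a PlayerStart actor, converts it to a transform and passes it to Respawn.
; Respawn spawns a new BP_PlayerCharacter there and has player controller 0 possess it.
; BeginPlay and ActorHasDied are empty.
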(event `self.ReceiveBeginPlay`)

(event `Event ActorHasDied`)

(fn `GameModeInterface`
  (returns (Success :type Boolean))
  (bind _playerstartcoord (`self.GetPlayerStart`))
  (`self.Respawn` (`KismetMathLibrary.Conv_VectorToTransform` _playerstartcoord))
  (return false))

(fn `GetPlayerStart`
  (returns (PlayerStartCoord :type "Vector Structure"))
  (bind _returnvalue (`GameplayStatics.GetActorOfClass` "/Script/Engine.PlayerStart"))
  (return (`self.K2_GetActorLocation` _returnvalue)))

(fn `Respawn`
  (params (`Respawn Transform` :type "Transform Structure"))
  (bind _returnvalue (`|SpawnActorFromClass` "/Game/MyContent/Blueprints/PlayerCharacter/BP_PlayerCharacter.BP_PlayerCharacter_C" `Respawn Transform` "Undefined" "OverrideRootScale" null null))
  (`Controller.Possess` (`GameplayStatics.GetPlayerController` 0) _returnvalue))

(fn `UserConstructionScript`)