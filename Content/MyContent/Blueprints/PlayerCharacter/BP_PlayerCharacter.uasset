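; BP_PlayerCharacter is the player character Blueprint, handling death and notifying the game mode when the character is destroyed.
; The kill interface event calls Die, which turns the mesh into a physics ragdoll and detaches the controller, then destroys the actor after a short delay.
; On Destroyed, it sends an interface message to the game mode if that implements BPI_GameModeInterface.
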(event `self.ReceiveBeginPlay`)

(event `/Game/MyContent/Blueprints/PlayerCharacter/Interfaces/BPI_KillCharacterInterface.KillCharacterInterface`
  (`self.Die`)
  (`KismetSystemLibrary.Delay` 2.0)
  (`self.K2_DestroyActor`))

(event `self.ReceiveDestroyed`
  (bind _returnvalue (`GameplayStatics.GetGameMode`))
  (if (`KismetSystemLibrary.DoesImplementInterface` _returnvalue "/Game/MyContent/Blueprints/PlayerCharacter/Interfaces/BPI_GameModeInterface.BPI_GameModeInterface_C")
    (message `/Game/MyContent/Blueprints/PlayerCharacter/Interfaces/BPI_GameModeInterface.GameModeInterface` _returnvalue)))

(fn `Die`
  (bind _mesh (`self.Mesh`))
  (`PrimitiveComponent.SetCollisionEnabled` (`self.Mesh`) "QueryAndPhysics")
  (`SkeletalMeshComponent.SetPhysicsBlendWeight` _mesh 1.0)
  (`PrimitiveComponent.SetSimulatePhysics` _mesh true)
  (`self.DetachFromControllerPendingDestroy`))

(fn `GameModeInterface`
  (returns (Success :type Boolean))
  (return false))

(fn `NewFunction`)

(fn `UserConstructionScript`)